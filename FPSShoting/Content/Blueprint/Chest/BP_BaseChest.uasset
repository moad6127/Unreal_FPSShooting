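; BP_BaseChest is the base chest actor Blueprint that opens a chest inventory screen for the player character that owns it.
; DisplayChest resolves the owner's controller and HUD, then asks the HUD for a widget controller built from the character's inventory component.
; It creates WBP_ChestInventory with that controller and the chest's own inventory component.
; It then adds the widget to the viewport, switches input to Game and UI, and shows the cursor.
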(event EventBeginPlay)

(event Collision|EventActorBeginOverlap
  (params (OtherActor :type Actor%20Object%20Reference)))

(event EventTick
  (params (DeltaSeconds :type Float%20%28single-precision%29)))

(event EventDisplayChest
  (bind _asbp_low_fpschracter (Utilities|Casting|CastToBP_LowFPSChracter (Components|GetOwner)))
  (bind _output_get (Variables|Default|SetBP_Character _asbp_low_fpschracter))
  (bind _asbp_fpscharacter_controller (Utilities|Casting|CastToBP_FPSCharacterController (Pawn|GetController _output_get)))
  (Variables|Default|SetPlayerController _asbp_fpscharacter_controller)
  (bind _asbp_fpshud (Utilities|Casting|CastToBP_FPSHUD (HUD|GetHUD (Variables|Default|GetPlayerController))))
  (Variables|Default|SetPlayerHUD _asbp_fpshud)
  (bind _returnvalue (Class|FPSHUD|MakeWidgetController (Variables|Default|GetPlayerHUD) (Utilities|Struct|MakeWidgetControllerParams (Variables|Default|GetPlayerController) (Variables|/Script/FPSCore.FPSCharacter|GetSInventoryComponent (Variables|Default|GetBP_Character)))))
  (Variables|Default|SetChestWidgetController _returnvalue)
  (bind _returnvalue_2 (UserInterface|CreateWidget "/Game/Blueprint/Widget/Widget/WBP_ChestInventory.WBP_ChestInventory_C" (Variables|Default|GetPlayerController)))
  (Variables|Default|SetChestWidget _returnvalue_2)
  (Variables|/Game/Blueprint/Widget/Widget/WBP_ChestInventory.WBP_ChestInventory_C|SetChestInventoryComp (Variables|Default|GetChestWidget) (Class|BaseChest|GetInventoryComponent))
  (Class|BasicWidget|SetWidgetController (Variables|Default|GetChestWidget) (Variables|Default|GetChestWidgetController))
  (UserInterface|Viewport|AddtoViewport (Variables|Default|GetChestWidget) 0)
  (Input|SetInputModeGameandUI (Variables|Default|GetPlayerController) (Variables|Default|GetChestWidget) "DoNotLock" true false)
  (Variables|/Script/Engine.PlayerController|SetbShowMouseCursor (Variables|Default|GetPlayerController) true))

(fn ConstructionScript)