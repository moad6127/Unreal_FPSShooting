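; BP_Target is a target actor that drops when it takes any damage and pops back up on its own.
; An Active flag, set at BeginPlay, ensures damage only triggers the down animation while the target is standing.
; Each hit clears the flag and starts a one-shot timer with a random delay of a few seconds, which plays the up animation and re-arms the target.
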(event Custom|OnTakeAnyDamage_이벤트
  (params (DamagedActor :type Actor%20Object%20Reference) (Damage :type Float%20%28single-precision%29) (DamageType :type Damage%20Type%20Object%20Reference) (InstigatedBy :type Controller%20Object%20Reference) (DamageCauser :type Actor%20Object%20Reference))
  (if (Variables|Default|GetActive)
    (Variables|Default|SetActive false)
    (Components|Animation|PlayAnimation (Variables|Default|GetMesh) "/Game/Asset/Target/Art/Environment/Damageables/A_Target_Down.A_Target_Down" false)
    (Utilities|Time|SetTimerbyEvent (delegate Custom|TargetUp) (Math|Random|RandomFloatinRange 1.0 5.0))))

(event Custom|TargetUp
  (Variables|Default|SetActive true)
  (Components|Animation|PlayAnimation (Variables|Default|GetMesh) "/Game/Asset/Target/Art/Environment/Damageables/A_Target_Up.A_Target_Up" false))

(event EventBeginPlay
  (EventDispatchers|AssignOnTakeAnyDamage (delegate Custom|OnTakeAnyDamage_이벤트))
  (Variables|Default|SetActive true))

(event Collision|EventActorBeginOverlap
  (params (OtherActor :type Actor%20Object%20Reference)))

(event EventTick
  (params (DeltaSeconds :type Float%20%28single-precision%29)))

(fn ConstructionScript)